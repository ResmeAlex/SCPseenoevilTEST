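; BP_SplineMove is a spline actor that, judging by its name, is meant for movement along a spline, though no movement logic exists yet.
; On BeginPlay it places SplineEnd at its closest spline point plus a Y offset, applying local-space results as world transforms.
; SplineEnd's rotation is sampled using the point count as index, and the player character is cached.
; BeginSpline and EndSpline are empty stubs.
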(event Custom|BeginSpline)

(event Custom|EndSpline)

(event EventBeginPlay
  (bind _splineend (Variables|Default|GetSplineEnd))
  (bind _splineend_2 (Variables|Default|GetSplineEnd))
  (bind _spline (Variables|Default|GetSpline))
  (bind _spline_2 (Variables|Default|GetSpline))
  (bind _returnvalue (Transformation|GetWorldLocation _splineend_2))
  (bind _returnvalue_2 (Spline|FindLocationClosesttoWorldLocation _spline_2 _returnvalue "Local"))
  (bind (_x _y _z) (Math|Vector|BreakVector _returnvalue_2))
  (Transformation|SetWorldLocation _splineend (Math|Vector|MakeVector _x (+ _y 5e+01) _z) false false)
  (Transformation|SetWorldRotation _splineend (Spline|GetRotationatSplinePoint _spline (Spline|GetNumberOfSplinePoints _spline) "Local") false false)
  (bind _ascharacter (Utilities|Casting|CastToCharacter (Game|GetPlayerCharacter 0)))
  (Variables|Default|SetPlayerRef _ascharacter))

(fn ConstructionScript)